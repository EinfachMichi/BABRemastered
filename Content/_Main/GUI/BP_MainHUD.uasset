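; Main HUD Blueprint that creates and manages the game's death, in-game, pause and tutorial widgets.
; On BeginPlay it adds all four to the viewport, with death and pause hidden and the tutorial visible.
; An event swaps the death and in-game screens by toggling visibility.
; Pause and resume events set game pause, pause-widget visibility, input mode and mouse cursor together.
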(event Custom|SetDeathGUIVisibility
  (params (Visibility :type Boolean))
  ;[0.05 0.05 0.05] SetDeathGUIVisibility
  (if Visibility
    (Widget|SetVisibility (Variables|Default|GetDeathGUI) "Visible")
    (Widget|SetVisibility (Variables|Default|GetInGameGUI) "Collapsed")
    (else
      (Widget|SetVisibility (Variables|Default|GetDeathGUI) "Collapsed")
      (Widget|SetVisibility (Variables|Default|GetInGameGUI) "Visible"))))

(event Custom|Pause%20Game
  (bind _returnvalue (Game|GetPlayerController 0))
  ;[0.05 0.05 0.05] Pause and resume
  (Game|SetGamePaused true)
  (Widget|SetVisibility (Variables|Default|GetGamePaused) "Visible")
  (Input|SetInputModeUIOnly _returnvalue (Variables|Default|GetGamePaused) "DoNotLock" false)
  (Variables|/Script/Engine.PlayerController|SetbShowMouseCursor _returnvalue true))

(event Custom|Resume%20Game
  (bind _returnvalue (Game|GetPlayerController 0))
  ;[0.05 0.05 0.05] Pause and resume
  (Game|SetGamePaused false)
  (Input|SetInputModeGameOnly _returnvalue false)
  (Widget|SetVisibility (Variables|Default|GetGamePaused) "Hidden")
  (Variables|/Script/Engine.PlayerController|SetbShowMouseCursor _returnvalue false))

(event EventBeginPlay
  ;[0.05 0.05 0.05] Begin Play
  (|AddWidgets))

(fn ConstructionScript)