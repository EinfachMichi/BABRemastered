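; BP_Weapon is a hitscan weapon that handles firing, reloading and reserve ammo.
; Fire spends a round and multi-traces objects from the player camera, damaging BP_Enemy hits by surface type and triggering BP_Furnace's AK and ammo buttons by component name.
; Reload plays a montage, then refills the clip from reserve ammo on completion.
; AddAmmo tops up the reserve, while Fire itself has no ammo or reload check.
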(event Custom|Reload
  ;[0.05 0.05 0.05] Reload
  (if (not (Math|Boolean|ORBoolean (Variables|Default|Get?Reloading) (== (Variables|Default|GetAmmo) (Variables|Default|GetMaxClipSize)) (<= (Variables|Default|GetTotalAmmo) 0)))
    (Variables|Default|Set?Reloading true)
    (Animation|Montage|PlayMontage (Variables|Default|GetSkeletalMesh) (Variables|Default|GetReloadAnimation)
      (:OnCompleted
        (Variables|Default|SetTempAmmo (Variables|Default|GetAmmo))
        (Variables|Default|SetAmmo (Math|Integer|SelectInt (Variables|Default|GetMaxClipSize) (+ (Variables|Default|GetAmmo) (Variables|Default|GetTotalAmmo)) (>= (+ (Variables|Default|GetAmmo) (Variables|Default|GetTotalAmmo)) (Variables|Default|GetMaxClipSize))))
        (Variables|Default|Set?Reloading false)
        (Variables|Default|SetTotalAmmo (Math|Integer|SelectInt (Math|Integer|Clamp(Integer) (- (Variables|Default|GetTotalAmmo) (- (Variables|Default|GetMaxClipSize) (Variables|Default|GetTempAmmo))) 0 (Variables|Default|GetTotalAmmo)) 0 (>= (+ (Variables|Default|GetAmmo) (Variables|Default|GetTotalAmmo)) (Variables|Default|GetMaxClipSize))))))))

(event Custom|AddAmmo
  (params (Ammo :type Integer))
  ;[0.05 0.05 0.05] Fire
  ;;[0.05 0.05 0.05] Add Ammo
  (Variables|Default|SetTotalAmmo (+ Ammo (Variables|Default|GetTotalAmmo))))

(event Custom|Fire
  (bind _returnvalue (Game|GetPlayerCharacter 0))
  (bind _asbp_player (Utilities|Casting|CastToBP_Player _returnvalue))
  (bind _firstpersoncamera (Variables|/Game/_Main/Character/Player/BP_Player.BP_Player_C|GetFirstPersonCamera _asbp_player))
  (bind _returnvalue_2 (Transformation|GetWorldLocation _firstpersoncamera))
  ;[0.05 0.05 0.05] Fire
  (Math|Integer|DecrementInt (Variables|Default|GetAmmo)
    (:%20%20
      (bind _outhits (Class|KismetSystemLibrary|LineTraceMultiforObjects _returnvalue_2 (+ _returnvalue_2 (* (Math|Vector|GetForwardVector (Transformation|GetWorldRotation _firstpersoncamera)) (Variables|Default|GetBulletDistance))) (Utilities|Array|MakeArray "ObjectTypeQuery1" "ObjectTypeQuery4") false (Utilities|Array|MakeArray (.AsBP%20Player (Utilities|Casting|CastToBP_Player (Game|GetPlayerCharacter 0)))) "None" true))
      (for _array_element _outhits
        (bind _asbp_enemy (Utilities|Casting|CastToBP_Enemy (.hitactor _array_element))
          (:then
            (Default|ReceiveDamage _asbp_enemy (Variables|/Script/PhysicsCore.PhysicalMaterial|GetSurfaceType (.physmat _array_element)) (Variables|Default|GetDamage) "0, 0, 0"))
          (:CastFailed
            (bind _asbp_furnace (Utilities|Casting|CastToBP_Furnace (.hitactor _array_element)))
            (bind _asstatic_mesh_component (Utilities|Casting|CastToStaticMeshComponent (.hitcomponent _array_element)))
            (if (Utilities|Enum|Equal(Enum) (Utilities|GetObjectName _asstatic_mesh_component) "AKButton")
              (Default|ButtonHit _asbp_furnace "AKButton")
              (elif (Utilities|Enum|Equal(Enum) (Utilities|GetObjectName _asstatic_mesh_component) "AmmoButton")
                (Default|ButtonHit _asbp_furnace "AmmoButton")))))))))

(fn ConstructionScript)