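; BP_Pistol is a semi-automatic pistol weapon Blueprint that fires one shot per trigger press.
; Shoot clears CanShoot and Release sets it again, so holding the trigger does not repeat fire.
; When not reloading, a shot with ammo plays the fire montage on the skeletal mesh and calls Fire, while an empty magazine plays a 2D sound.
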(event EventShoot
  ;[0.05 0.05 0.05] Shoot
  (if (Variables|Default|GetCanShoot)
    (Variables|Default|SetCanShoot false)
    (if (not (Variables|Default|Get?Reloading))
      (if (> (Variables|Default|GetAmmo) 0)
        (Components|Animation|PlayAnimation (Variables|Default|GetSkeletalMesh) "/Game/_Main/Weapons/Pistols/Animation/Pistol_Fire_Montage.Pistol_Fire_Montage" false)
        (CallFunction|Fire)
        (else
          ;;[0.9583 0 0] Empty Magazine Sound
          (Audio|PlaySound2D (Variables|Default|GetEmptyMagazineSound) 1.0 1.0 0.0 0 0))))))

(event EventRelease
  ;[0.05 0.05 0.05] Release
  (Variables|Default|SetCanShoot true))

(fn ConstructionScript
  (|CallParentFunction))