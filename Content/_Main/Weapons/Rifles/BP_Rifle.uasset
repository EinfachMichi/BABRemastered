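; Rifle weapon Blueprint that handles trigger press and release for firing.
; Shoot is gated by CanShoot and Reloading; with ammo it starts a montage, calls Fire immediately, then re-arms after a ShootCooldown delay.
; An empty magazine plays a click sound and re-arms at once.
; Release also re-arms CanShoot, so letting go of the trigger can bypass the remaining cooldown.
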(event EventShoot
  ;[0.05 0.05 0.05] Shoot
  (if (Variables|Default|GetCanShoot)
    (if (not (Variables|Default|Get?Reloading))
      (Variables|Default|SetCanShoot false)
      (if (> (Variables|Default|GetAmmo) 0)
        ;;[1 0 0] Fire Animation
        (Animation|Montage|PlayMontage (Variables|Default|GetSkeletalMesh) 0
          (:then
            (CallFunction|Fire)
            (Utilities|FlowControl|Delay (Variables|Default|GetShootCooldown))))
        (else
          ;;[0.9583 0 0] Empty Magazine Sound
          (Audio|PlaySound2D (Variables|Default|GetEmptyMagazineSound) 1.0 1.0 0.0 0 0)))
      (Variables|Default|SetCanShoot true))))

(event EventRelease
  ;[0.05 0.05 0.05] Release
  (if (not (Variables|Default|GetCanShoot))
    (Variables|Default|SetCanShoot true)))

(fn ConstructionScript
  (|CallParentFunction))