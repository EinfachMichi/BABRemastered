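; BP_Default is the default zombie enemy, a child Blueprint that supplies the melee Attack event against the player.
; Attack plays the zombie attack montage only while the player is alive, setting the cooldown flag and calling AttackPlayer from the montage notify.
; On completion or interruption it changes State, waits out AttackCooldown, clears the flag and calls FollowPlayer to resume the chase.
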(event EventAttack
  ;[0.05 0.05 0.05] Attack
  (bind _asbp_player (Utilities|Casting|CastToBP_Player (Game|GetPlayerCharacter 0)))
  (if (not (Variables|/Game/_Main/Character/Player/BP_Player.BP_Player_C|GetIsDead _asbp_player))
    (Animation|Montage|PlayMontage (Variables|Character|GetMesh) "/Game/_Main/Character/Enemy/Default/Animations/Default_Zombie_Attack_Montage.Default_Zombie_Attack_Montage"
      (:then
        (Variables|Default|Set?AttackOnCooldown true))
      (:OnCompleted
        (Variables|Default|SetState "NewEnumerator2" :!label _label)
        (Utilities|FlowControl|Delay (Variables|Default|GetAttackCooldown))
        (Variables|Default|Set?AttackOnCooldown false)
        (CallFunction|FollowPlayer))
      (:OnInterrupted
        (goto _label))
      (:OnNotifyBegin
        (CallFunction|AttackPlayer)))))

(fn ConstructionScript
  (|CallParentFunction))