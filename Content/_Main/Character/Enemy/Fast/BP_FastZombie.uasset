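; BP_FastZombie is the fast zombie enemy, defining its attack and hit reaction on top of inherited behavior.
; Attack checks that the player is alive, plays sound and montage, calls AttackPlayer on the montage notify, then resumes FollowPlayer on completion.
; OnHit is ignored mid-attack; otherwise it halts movement during the reaction montage, then restores NavWalking and pursuit unless State equals the enum's first entry.
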(event EventOnHit
  (if (not (Variables|Default|Get?Attacking))
    (Pawn|Components|CharacterMovement|DisableMovement (Variables|Character|GetCharacterMovement))
    (Animation|Montage|PlayMontage (Variables|Character|GetMesh) "/Game/_Main/Character/Enemy/Default/Animations/Default_Zombie_Reaction_Hit_Montage.Default_Zombie_Reaction_Hit_Montage"
      (:OnCompleted
        (if (not (Utilities|Enum|Equal(Enum) (Variables|Default|GetState) "NewEnumerator0"))
          (Pawn|Components|CharacterMovement|SetMovementMode (Variables|Character|GetCharacterMovement) "MOVE_NavWalking" 0)
          (CallFunction|FollowPlayer))))))

(event EventAttack
  (bind _zombie_sound (Variables|Default|GetZombie%20Sound))
  ;[0.05 0.05 0.05] Attack
  (bind _asbp_player (Utilities|Casting|CastToBP_Player (Game|GetPlayerCharacter 0)))
  (if (not (Variables|/Game/_Main/Character/Player/BP_Player.BP_Player_C|GetIsDead _asbp_player))
    (Variables|Default|Set?Attacking true)
    (Audio|Components|Audio|SetSound _zombie_sound (Variables|Default|GetAttackSound))
    (Audio|Components|Audio|Play _zombie_sound 0.0)
    (Animation|Montage|PlayMontage (Variables|Character|GetMesh) "/Game/_Main/Character/Enemy/Default/Animations/Default_Zombie_Attack_Montage.Default_Zombie_Attack_Montage"
      (:OnCompleted
        (Variables|Default|Set?Attacking false)
        (CallFunction|FollowPlayer))
      (:OnNotifyBegin
        (CallFunction|AttackPlayer)))))

(fn ConstructionScript
  (|CallParentFunction))