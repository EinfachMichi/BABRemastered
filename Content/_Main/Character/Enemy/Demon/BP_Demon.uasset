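; BP_Demon is a demon enemy character that supplies its own attack and hit-reaction events on top of inherited enemy logic.
; Attack plays a zombie attack montage while the player is alive, with a montage notify triggering AttackPlayer.
; When the montage completes or is interrupted, it resumes following the player, changes state and holds an attack cooldown flag for a delay.
; OnHit calls PlayMontage on the mesh with no montage specified.
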(event EventOnHit
  ;[0.05 0.05 0.05] On Hit
  ;;[1 0 0] Hit Animation
  (Animation|Montage|PlayMontage (Variables|Character|GetMesh) 0))

(event EventAttack
  ;[0.05 0.05 0.05] Attack
  (bind _asbp_player (Utilities|Casting|CastToBP_Player (Game|GetPlayerCharacter 0)))
  (if (not (Variables|/Game/_Main/Character/Player/BP_Player.BP_Player_C|GetIsDead _asbp_player))
    (Animation|Montage|PlayMontage (Variables|Character|GetMesh) "/Game/_Main/Character/Enemy/Demon/Animations/Template_Zombie_Attack_Montage.Template_Zombie_Attack_Montage"
      (:OnCompleted
        (CallFunction|FollowPlayer :!label _label)
        (Variables|Default|Set?AttackOnCooldown true)
        (Variables|Default|SetState "NewEnumerator2")
        (Utilities|FlowControl|Delay (Variables|Default|GetAttackCooldown))
        (Variables|Default|Set?AttackOnCooldown false))
      (:OnInterrupted
        (goto _label))
      (:OnNotifyBegin
        (CallFunction|AttackPlayer)))))

(fn ConstructionScript
  (|CallParentFunction))