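; BP_Demon is a demon enemy that defines the attack, hit and death animation behavior for that character.
; Attack plays a montage whose notify calls AttackPlayer, so the attack is timed to the animation.
; When the montage completes or is interrupted, it calls FollowPlayer and then waits for the attack cooldown.
; OnHit and OnDeath each only play a montage on the mesh.
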(event EventOnHit
  ;[0.05 0.05 0.05] On Hit
  ;;[1 0 0] Hit Animation
  (Animation|Montage|PlayMontage (Variables|Character|GetMesh) 0))

(event EventOnDeath
  ;[0.05 0.05 0.05] On Death
  ;;[1 0 0] Death Animation
  (Animation|Montage|PlayMontage (Variables|Character|GetMesh) 0))

(event EventAttack
  ;[0.05 0.05 0.05] Attack
  ;;[1 0 0] Attack Animation
  (Animation|Montage|PlayMontage (Variables|Character|GetMesh) 0
    (:OnCompleted
      (CallFunction|FollowPlayer :!label _label)
      (Utilities|FlowControl|Delay (Variables|Default|GetAttackCooldown)))
    (:OnInterrupted
      (goto _label))
    (:OnNotifyBegin
      (CallFunction|AttackPlayer))))

(fn ConstructionScript
  (|CallParentFunction))