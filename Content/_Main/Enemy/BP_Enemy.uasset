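; BP_Enemy is an enemy character that patrols, chases and attacks the player, with health and death handling.
; A randomized looping timer drives patrol moves to random reachable points.
; Overlapping the construction-scaled sight sphere starts a faster chase through a recursive AI MoveTo loop that calls Attack when off cooldown.
; AttackPlayer damages players via sphere overlap, while incoming damage is scaled by head, body or limb surface type.
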(event OnComponentBeginOverlap(SightRangeCollision)
  (params (OverlappedComponent :type Primitive%20Component%20Object%20Reference) (OtherActor :type Actor%20Object%20Reference) (OtherComp :type Primitive%20Component%20Object%20Reference) (OtherBodyIndex :type Integer) (bFromSweep :type Boolean) (SweepResult :type Hit%20Result%20Structure%20%28by%20ref%29))
  ;[0.05 0.05 0.05] On Sight Range Entered
  (Utilities|Casting|CastToBP_Player OtherActor)
  (Variables|/Script/Engine.CharacterMovementComponent|SetMaxWalkSpeed (Variables|Character|GetCharacterMovement) (Variables|Default|GetChaseSpeed))
  (Variables|Default|SetState "NewEnumerator2")
  (CallFunction|FollowPlayer))

(event Custom|FollowPlayer
  ;[0.05 0.05 0.05] Follow Player
  (if (Utilities|Enum|NotEqual(Enum) (Variables|Default|GetState) "NewEnumerator0")
    (AI|AIMoveTo self "0, 0, 0" (Game|GetPlayerController 0) (Variables|Default|GetStoppingDistance) false
      (:OnSuccess
        (if (Variables|Default|Get?AttackOnCooldown)
          (CallFunction|FollowPlayer :!label _label)
          (else
            (CallFunction|Attack))))
      (:OnFail
        (goto _label)))))

(event Custom|Patrol
  ;[0.05 0.05 0.05] Patrol
  (if (Utilities|Enum|Equal(Enum) (Variables|Default|GetState) "NewEnumerator1")
    (AI|AIMoveTo self (CallFunction|GetRandomLocationinRange) 0 5.0 false)))

(event Custom|ReceiveDamage
  (params (SurfaceType :type EPhysicalSurface%20Enum :default "SurfaceType_Default") (Damage :type Float%20%28double-precision%29) (Hit%20Location :type Vector))
  ;[0.05 0.05 0.05] Receive Damage
  (if (not (Utilities|Enum|NotEqual(Enum) (Variables|Default|GetState) "NewEnumerator0"))
    (switch Utilities|FlowControl|Switch|SwitchonEPhysicalSurface SurfaceType
      (:SurfaceType_Default
        (Variables|Default|SetDamageMultiplier (Variables|Default|GetLimbsMultiplier) :!label _label))
      (:SurfaceType1
        (goto _label))
      (:SurfaceType2
        (Variables|Default|SetDamageMultiplier (Variables|Default|GetBodyMultiplier)))
      (:SurfaceType3
        (Variables|Default|SetDamageMultiplier (Variables|Default|GetHeadMultiplier))))
    (CallFunction|Hit (Variables|Default|GetDamageMultiplier) Damage)
    (CallFunction|OnHit)))

(event Custom|Hit
  (params (Multiplier :type Float%20%28double-precision%29) (Damage :type Float%20%28double-precision%29))
  ;[0.05 0.05 0.05] Hit
  (if (<= (- (Variables|Default|GetHealth) (* Multiplier Damage)) 0.0)
    (CallFunction|Death)
    (else
      (Variables|Default|SetHealth (- (Variables|Default|GetHealth) (* Multiplier Damage))))))

(event Custom|Death
  ;[0.05 0.05 0.05] Death
  (if (Utilities|Enum|NotEqual(Enum) (Variables|Default|GetState) "NewEnumerator0")
    (Variables|Default|SetState "NewEnumerator0")
    (Components|Movement|StopMovementImmediately (Variables|Character|GetCharacterMovement))
    (Collision|SetCollisionEnabled (Variables|Collision|GetCapsuleComponent) "NoCollision")))

(event Custom|AttackPlayer
  ;[0.05 0.05 0.05] Attack Player
  (bind (_outactors _returnvalue) (Collision|SphereOverlapActors (Transformation|GetWorldLocation (Variables|Default|GetAttackPoint)) (Variables|Default|GetAttackRadius) (Utilities|Array|MakeArray "ObjectTypeQuery3") "/Game/_Main/Player/BP_Player.BP_Player_C" (Utilities|Array|MakeArray self)))
  (if _returnvalue
    (for _array_element _outactors
      (bind _asbp_player (Utilities|Casting|CastToBP_Player _array_element))
      (Default|ReceiveDamage _asbp_player (Variables|Default|GetDamage)))))

(event EventBeginPlay
  ;[0.05 0.05 0.05] Begin Play
  (|InitializeValues)
  (Utilities|Time|SetTimerbyEvent (delegate Custom|Patrol) (Math|Random|RandomFloatinRange (Variables|Default|GetPatrolCycleMin) (Variables|Default|GetPatrolCycleMax)) true))

(fn ConstructionScript
  (bind _sightrangecollision (Variables|Default|GetSightRangeCollision))
  (Transformation|SetWorldScale3D _sightrangecollision (* (.scale (Transformation|GetRelativeTransform _sightrangecollision)) (/ (* (Variables|Default|GetSightRange) 2.0) 5e+01))))

(fn GetRandomLocationinRange
  (return (.RandomLocation (AI|Navigation|GetRandomReachablePointinRadius (Transformation|GetActorLocation) (Variables|Default|GetPatrolRadius) 0 0))))