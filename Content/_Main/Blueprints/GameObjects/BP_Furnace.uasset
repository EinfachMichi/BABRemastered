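; BP_Furnace is a shop that destroys enemies entering its burn radius, banks random ash, and sells AK pickups and ammo boxes.
; ButtonHit takes a button name, spawns the item at a spawn point and deducts ash if that button is enabled.
; Button materials show availability from ash, GameInstance HasAK and CanSpawnAK, which locks ammo until an AK is bought.
; Adding ash refreshes buttons only upon reaching the cap.
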(event OnComponentBeginOverlap(BurnRadius)
  (params (OverlappedComponent :type Primitive%20Component%20Object%20Reference) (OtherActor :type Actor%20Object%20Reference) (OtherComp :type Primitive%20Component%20Object%20Reference) (OtherBodyIndex :type Integer) (bFromSweep :type Boolean) (SweepResult :type Hit%20Result%20Structure%20%28by%20ref%29))
  ;[0.05 0.05 0.05] Burn Enemy
  (bind _asbp_enemy (Utilities|Casting|CastToBP_Enemy OtherActor))
  (Actor|DestroyActor _asbp_enemy)
  (CallFunction|AddAsh (Math|Random|RandomFloatinRange (Variables|Default|GetMinAshValue) (Variables|Default|GetMaxAshValue))))

(event Custom|UpdateFurnace
  ;[0.05 0.05 0.05] Update Furnace
  (|UpdateAKButton)
  (|UpdateAmmoButton))

(event Custom|ButtonHit
  (params (Name :type Name))
  (if (== Name "AKButton")
    (if (Variables|Default|GetAKButtonShootable)
      (Variables|Default|SetCanSpawnAK false)
      (Game|SpawnActorfromClass "/Game/_Main/Blueprints/GameObjects/BP_AKPickup.BP_AKPickup_C" (Math|Conversions|ToTransform(Vector) (Transformation|GetWorldLocation (Variables|Default|GetItem%20Spawnpoint))) "AlwaysSpawn" "MultiplyWithRoot" 0 0)
      (Variables|Default|SetAsh (- (Variables|Default|GetAsh) (Variables|Default|GetAKCost)))
      (CallFunction|UpdateFurnace :!label _label))
    (elif (== Name "AmmoButton")
      (if (Variables|Default|GetAmmoButtonShootable)
        (Game|SpawnActorfromClass "/Game/_Main/Blueprints/Interactables/AmmoBox/9mm/BP_9mmAmmoBox.BP_9mmAmmoBox_C" (Math|Conversions|ToTransform(Vector) (Transformation|GetWorldLocation (Variables|Default|GetItem%20Spawnpoint))) "AlwaysSpawn" "MultiplyWithRoot" 0 0)
        (Variables|Default|SetAsh (- (Variables|Default|GetAsh) (Variables|Default|GetAmmoCost)))
        (goto _label)))))

(event Custom|AddAsh
  (params (Value :type Float%20%28double-precision%29))
  ;[0.05 0.05 0.05] Add Ash
  (bind _output_get (Variables|Default|SetAsh (+ Value (Variables|Default|GetAsh))))
  (if (>= _output_get (Variables|Default|GetMaxAsh))
    (Variables|Default|SetAsh (Variables|Default|GetMaxAsh))
    (CallFunction|UpdateFurnace)))

(event EventBeginPlay
  ;[0.05 0.05 0.05] Begin Play
  (CallFunction|UpdateFurnace))

(fn ConstructionScript)