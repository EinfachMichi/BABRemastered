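; BP_WaterPump is an interactable water pump that gradually heals the player while they stand near it.
; Interacting starts the Timer timeline, which adds health each tick, scaled by delta time to HealValue per three seconds, whenever the player is inside the HealingRange sphere.
; Interaction locks until the timeline finishes and a cooldown elapses.
; The construction script sizes the sphere from HealingRadius.
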(event OnComponentBeginOverlap(HealingRange)
  (params (OverlappedComponent :type Primitive%20Component%20Object%20Reference) (OtherActor :type Actor%20Object%20Reference) (OtherComp :type Primitive%20Component%20Object%20Reference) (OtherBodyIndex :type Integer) (bFromSweep :type Boolean) (SweepResult :type Hit%20Result%20Structure%20%28by%20ref%29))
  ;[0.05 0.05 0.05] Player in range management
  (Utilities|Casting|CastToBP_Player OtherActor)
  (Variables|Default|Set?InRange true))

(event OnComponentEndOverlap(HealingRange)
  (params (OverlappedComponent :type Primitive%20Component%20Object%20Reference) (OtherActor :type Actor%20Object%20Reference) (OtherComp :type Primitive%20Component%20Object%20Reference) (OtherBodyIndex :type Integer))
  ;[0.05 0.05 0.05] Player in range management
  (Utilities|Casting|CastToBP_Player OtherActor)
  (Variables|Default|Set?InRange false))

(event EventInteract
  ;[0.05 0.05 0.05] Interact
  (if (Variables|Default|GetCanInteract)
    (Variables|Default|SetCanInteract false)
    (Timeline|Timer PlayFromStart
      (:Update
        (if (Variables|Default|Get?InRange)
          (bind _asbp_player (Utilities|Casting|CastToBP_Player (Game|GetPlayerCharacter 0)))
          (Default|AddHealth _asbp_player (* (Utilities|Time|GetWorldDeltaSeconds) (/ (Variables|Default|GetHealValue) 3.0)))))
      (:Finished
        (Utilities|FlowControl|Delay (Variables|Default|GetInteractionCooldown))
        (Variables|Default|SetCanInteract true)))))

(fn ConstructionScript
  (Components|Sphere|SetSphereRadius (Variables|Default|GetHealingRange) (Variables|Default|GetHealingRadius) false))