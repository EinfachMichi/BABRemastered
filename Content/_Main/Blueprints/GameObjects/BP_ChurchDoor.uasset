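; BP_ChurchDoor is a church door that opens and closes by toggling its static mesh's visibility and collision.
; When BP_Player first overlaps the trigger sphere, the door closes behind a one-time Triggered flag.
; That same overlap then tells the BP_StoryMode game mode to start its timer.
; Open is exposed as an event but is not called within this Blueprint.
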(event OnComponentBeginOverlap(TriggerSphere)
  (params (OverlappedComponent :type Primitive%20Component%20Object%20Reference) (OtherActor :type Actor%20Object%20Reference) (OtherComp :type Primitive%20Component%20Object%20Reference) (OtherBodyIndex :type Integer) (bFromSweep :type Boolean) (SweepResult :type Hit%20Result%20Structure%20%28by%20ref%29))
  ;[0.05 0.05 0.05] Trigger Sphere Triggered
  (if (not (Variables|Default|Get?Triggered))
    (Utilities|Casting|CastToBP_Player OtherActor)
    (CallFunction|Close)
    (Variables|Default|Set?Triggered true)
    (bind _asbp_story_mode (Utilities|Casting|CastToBP_StoryMode (Game|GetGameMode)))
    (Default|StartTimer _asbp_story_mode)))

(event Custom|Open
  ;[0.05 0.05 0.05] Toggle Door
  (Rendering|SetVisibility (Variables|Default|GetStaticMesh) false false)
  (Collision|SetCollisionEnabled (Variables|Default|GetStaticMesh) "NoCollision"))

(event Custom|Close
  ;[0.05 0.05 0.05] Toggle Door
  (Rendering|SetVisibility (Variables|Default|GetStaticMesh) true false)
  (Collision|SetCollisionEnabled (Variables|Default|GetStaticMesh) "QueryAndPhysics"))

(fn ConstructionScript)