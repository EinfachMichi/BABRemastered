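; BP_SpawnManager supplies spawn locations from the spawn points and spawn spheres placed in the level.
; On BeginPlay it caches every BP_SpawnPoint position as an unoccupied entry and collects all BP_SpawnSphere actors.
; GetRandomSpawnLocation returns the first unoccupied point, otherwise a random location from a randomly chosen sphere.
; Nothing here marks points as occupied.
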(event EventBeginPlay
  ;[0.05 0.05 0.05] Get all spawnpoints
  (Utilities|FlowControl|Sequence
    (:then_0
      (bind _outactors (Actor|GetAllActorsOfClass "/Game/_Main/Blueprints/SpawnSystem/BP_SpawnPoint.BP_SpawnPoint_C"))
      (for _array_element _outactors
        (Utilities|Array|Add (Variables|Default|GetSpawnLocations) (Utilities|Struct|MakeS_SpawnLocation (Transformation|GetActorLocation _array_element) false))))
    (:then_1
      (bind _outactors_2 (Actor|GetAllActorsOfClass "/Game/_Main/Blueprints/SpawnSystem/BP_SpawnSphere.BP_SpawnSphere_C"))
      (for _array_element_2 _outactors_2
        (Utilities|Array|Add (Variables|Default|GetSpawnSpheres) _array_element_2)))))

(fn ConstructionScript)

(fn GetRandomSpawnLocation
  (bind _array_element (Utilities|Array|ForEachLoopwithBreak (Variables|Default|GetSpawnLocations) :!label _label)
    (:LoopBody
      (if (not (.occupied _array_element))
        (LocalVariables|SetTempLocation (.location _array_element))
        (LocalVariables|SetSpawnPointFound true)
        (goto _label Break)))
    (:Completed
      (if (LocalVariables|GetSpawnPointFound)
        _
        (else
          (bind _location (Default|GetRandomLocation (Utilities|Array|Get(acopy) (Variables|Default|GetSpawnSpheres) (Math|Random|RandomIntegerinRange 0 (- (Utilities|Array|Length (Variables|Default|GetSpawnSpheres)) 1)))))
          (LocalVariables|SetTempLocation _location)))
      (return (LocalVariables|GetTempLocation)))))