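; BP_SpawnSphere is a spawn volume that defines a circular area for picking random spawn locations.
; Its construction script scales the Sphere component by twice the Radius variable to visualize that area.
; GetRandomLocation returns a random navigation-reachable point within Radius of the actor's location.
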(fn ConstructionScript
  (bind _sphere (Variables|Default|GetSphere))
  (Transformation|SetRelativeScale3D _sphere (* (.scale (Transformation|GetRelativeTransform _sphere)) (* (Variables|Default|GetRadius) 2.0))))

(fn GetRandomLocation
  (return (.RandomLocation (AI|Navigation|GetRandomReachablePointinRadius (Transformation|GetActorLocation) (Variables|Default|GetRadius) 0 0))))