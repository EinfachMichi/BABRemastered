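; Boss trigger volume that ends the game when the player walks into it.
; An overlap of the Box by the BP_Player capsule disables player input and plays the Scream component.
; After a short delay, it calls TriggerEnd on the EndGame member of BP_MainHUD.
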(event OnComponentBeginOverlap(Box)
  (params (OverlappedComponent :type Primitive%20Component%20Object%20Reference) (OtherActor :type Actor%20Object%20Reference) (OtherComp :type Primitive%20Component%20Object%20Reference) (OtherBodyIndex :type Integer) (bFromSweep :type Boolean) (SweepResult :type Hit%20Result%20Structure%20%28by%20ref%29))
  (bind _asbp_player (Utilities|Casting|CastToBP_Player OtherActor))
  (if (== OtherComp (Variables|/Script/Engine.Character|GetCapsuleComponent _asbp_player))
    (Input|DisableInput (Game|GetPlayerCharacter 0) (Game|GetPlayerController 0))
    (Audio|Components|Audio|Play (Variables|Default|GetScream) 0.0)
    (Utilities|FlowControl|Delay 2.0)
    (bind _asbp_main_hud (Utilities|Casting|CastToBP_MainHUD (HUD|GetHUD (Game|GetPlayerController 0))))
    (Default|TriggerEnd (Variables|/Game/_Main/GUI/BP_MainHUD.BP_MainHUD_C|GetEndGame _asbp_main_hud))))

(fn ConstructionScript)