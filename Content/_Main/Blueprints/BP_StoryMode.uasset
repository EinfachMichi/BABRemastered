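; BP_StoryMode runs story mode by loading the current day's level and spawning that day's enemy wave.
; On BeginPlay it compares the current level name with the day data's level, opens a level on a mismatch, then calls StartDay.
; StartDay finds the BP_SpawnManager and triggers SpawnWave, which loops over the wave count, spawning the configured enemy class at random manager-provided locations.
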(event Custom|StartDay
  ;[0.05 0.05 0.05] Start Day
  (bind _returnvalue (Actor|GetActorOfClass "/Game/_Main/Blueprints/SpawnSystem/BP_SpawnManager.BP_SpawnManager_C"))
  (Variables|Default|SetSpawnManager _returnvalue)
  (CallFunction|SpawnWave))

(event Custom|SpawnWave
  (bind _data (Utilities|GetCurrentDayData))
  (bind _wave (Variables|/Game/_Main/Blueprints/WaveSystem/BPDA_Day.BPDA_Day_C|GetWave _data))
  ;[0.05 0.05 0.05] Spawn Wave
  (for _index (range 0 (Variables|/Game/_Main/Blueprints/WaveSystem/BPDA_Wave.BPDA_Wave_C|GetCount _wave))
    (Game|SpawnActorfromClass (Variables|/Game/_Main/Blueprints/WaveSystem/BPDA_Wave.BPDA_Wave_C|GetEnemy _wave) (Math|Conversions|ToTransform(Vector) (Default|GetRandomSpawnLocation (Variables|Default|GetSpawnManager))) "AlwaysSpawn" "MultiplyWithRoot" 0 0)))

(event Custom|OpenLevel
  ;[0.05 0.05 0.05] Open Level
  (Game|OpenLevel(byName) (Variables|/Game/_Main/Blueprints/WaveSystem/BPDA_Day.BPDA_Day_C|GetLevelName (Utilities|GetCurrentDayData))))

(event EventBeginPlay
  ;[0.05 0.05 0.05] Begin Play
  (bind _returnvalue (Game|GetCurrentLevelName true))
  (if (Utilities|Enum|Equal(Enum) _returnvalue (Utilities|String|ToString(Name) (Variables|/Game/_Main/Blueprints/WaveSystem/BPDA_Day.BPDA_Day_C|GetLevelName (Utilities|GetCurrentDayData))))
    _
    (else
      (CallFunction|OpenLevel)))
  (CallFunction|StartDay))

(fn ConstructionScript)